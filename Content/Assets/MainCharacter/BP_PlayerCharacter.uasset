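; Player character Blueprint for a cat that aims down sights, throws kunai and interacts.
; Right mouse toggles aim while held, adding the crosshair widget created at BeginPlay to the viewport and removing it on release.
; F or left mouse calls ShootKunai and E calls Interact, with this logic defined outside the graph.
; Tick polls movement input to set CanRun on the Cat_ABP animation Blueprint.
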(event `self.ReceiveBeginPlay`
  ;[1 1 1] Create the crosshair widget and store it as a variable
  (bind _returnvalue (`|CreateWidget` "/Game/Blueprints/Widgets/WBP_Crosshair.WBP_Crosshair_C" (`GameplayStatics.GetPlayerController` 0)))
  (set `self.CrosshairWiget` _returnvalue))

(event `Key|RightMouseButton`
  (params (Key :type "Key Structure"))
  (bind _crosshairwiget (`self.CrosshairWiget`))
  (bind _crosshairwiget_2 (`self.CrosshairWiget`))
  ;[1 1 1] Zoom in and zoom out for aim down sight with showing the crosshair
  (:`Pressed`
    (`self.AimDownSight`)
    (`/Engine/EditorBlueprintResources/StandardMacros.IsValid` _crosshairwiget
      (:`Is Valid`
        (`UserWidget.AddToViewport` _crosshairwiget_2 0))))
  (:`Released`
    (`self.ExitAimDownSight`)
    (`/Engine/EditorBlueprintResources/StandardMacros.IsValid` _crosshairwiget
      (:`Is Valid`
        (`Widget.RemoveFromParent` _crosshairwiget_2)))))

(event `Key|F`
  (params (Key :type "Key Structure"))
  ;[1 1 1] Launch shuriken
  (:`Pressed`
    (`self.ShootKunai` :!label _label)))

(event `Key|E`
  (params (Key :type "Key Structure"))
  ;[1 1 1] Interaction Button
  (:`Pressed`
    (`self.Interact`)))

(event `Key|LeftMouseButton`
  (params (Key :type "Key Structure"))
  ;[1 1 1] Launch shuriken
  (:`Pressed`
    (goto _label)))

(event `self.ReceiveTick`
  (params (DeltaSeconds :type "Float (single-precision)"))
  (bind _returnvalue (`SkeletalMeshComponent.GetAnimInstance` (`self.Mesh`)))
  ;[1 1 1] Move
  (if (or (!= (`self.GetInputAxisValue`) 0.0) (!= (`self.GetInputAxisValue`) 0.0))
    (bind _ascat_abp (cast `/Game/Assets/MainCharacter/Cat_ABP` _returnvalue))
    (set `/Game/Assets/MainCharacter/Cat_ABP.CanRun` true _ascat_abp)
    (else
      (bind _ascat_abp_2 (cast `/Game/Assets/MainCharacter/Cat_ABP` _returnvalue))
      (set `/Game/Assets/MainCharacter/Cat_ABP.CanRun` false _ascat_abp_2))))

(fn `UserConstructionScript`)