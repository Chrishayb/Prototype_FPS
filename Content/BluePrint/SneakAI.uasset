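; SneakAI is an AI controller that possesses an EnemyMele guard and runs SneakTree for stealth-style detection of the player.
; Perception updates set CanSeePlayer on the blackboard, ignoring hidden players, and raise Alert on a sighting.
; Walk, Run, Alert and Looking events forward to the guard.
; Run records the player's location one second after sight is lost, and repeated Alert calls count down to clearing the Alert flag.
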(event `self.AIPerception.OnTargetPerceptionUpdated`
  (params (Actor :type "Actor Object Reference") (Stimulus :type "AIStimulus Structure"))
  (bind _asbp_player_character (cast `/Game/Blueprints/BP_PlayerCharacter` Actor))
  (bind _returnvalue (and (not (`/Game/Blueprints/BP_PlayerCharacter.isHidden` _asbp_player_character)) (`.bSuccessfullySensed` (break `AIStimulus` Stimulus))))
  (`BlackboardComponent.SetValueAsBool` (`AIBlueprintHelperLibrary.GetBlackboard` null) "CanSeePlayer" _returnvalue)
  (if _returnvalue
    (bind _blackboardcomponent (`self.UseBlackboard` "/Game/BluePrint/SneakBoard.SneakBoard"))
    (`BlackboardComponent.SetValueAsBool` _blackboardcomponent "Alert" true)))

(event `Walk`
  (`/Game/BluePrint/EnemyMele.Walk` (`self.Guard`)))

(event `Run`
  (`/Game/BluePrint/EnemyMele.Run` (`self.Guard`))
  (if (not (`.bSuccessfullySensed` (break `AIStimulus` (stale `self.AIPerception.OnTargetPerceptionUpdated` Stimulus))))
    (`KismetSystemLibrary.Delay` 1.0)
    (bind _blackboardcomponent (`self.UseBlackboard` "/Game/BluePrint/SneakBoard.SneakBoard"))
    (`BlackboardComponent.SetValueAsVector` _blackboardcomponent "LastKnownPlayerLocation" (`self.K2_GetActorLocation` (`GameplayStatics.GetPlayerCharacter` 0)))))

(event `Alert`
  (`/Game/BluePrint/EnemyMele.Alert` (`self.Guard`))
  (bind _result (`/Engine/EditorBlueprintResources/StandardMacros.DecrementInt` (`self.StopSeekCount`))
    (:`  `
      (if (<= _result 0)
        (bind _blackboardcomponent (`self.UseBlackboard` "/Game/BluePrint/SneakBoard.SneakBoard"))
        (`BlackboardComponent.SetValueAsBool` _blackboardcomponent "Alert" false)
        (set `self.StopSeekCount` 2)))))

(event `Looking`
  (`/Game/BluePrint/EnemyMele.Looking` (`self.Guard`)))

(event `self.OnPossess`
  (params (PossessedPawn :type "Pawn Object Reference"))
  (bind _asenemy_mele (cast `/Game/BluePrint/EnemyMele` PossessedPawn))
  (set `self.Guard` _asenemy_mele)
  (`self.RunBehaviorTree` "/Game/BluePrint/SneakTree.SneakTree"))

(fn `UserConstructionScript`)