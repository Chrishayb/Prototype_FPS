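; Shuriken is a thrown projectile actor that flies forward under physics and stops where it hits.
; On BeginPlay it applies a one-time forward impulse, scaled by ProjectileSpeed, to its placeholder TEMPmesh.
; When the mesh hits anything, its hit event compares the mesh's HitComponent against the player character, then zeroes velocity and disables physics simulation, freezing it in place.
; No damage logic is present.
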(event `self.ReceiveBeginPlay`
  (`PrimitiveComponent.AddImpulse` (`self.TEMPmesh`) (* (`KismetMathLibrary.GetForwardVector` (`self.K2_GetActorRotation`)) (`self.ProjectileSpeed`)) "None" false))

(event `self.TEMPmesh.OnComponentHit`
  (params (HitComponent :type "PrimitiveComponent Object Reference") (OtherActor :type "Actor Object Reference") (OtherComp :type "PrimitiveComponent Object Reference") (NormalImpulse :type "Vector Structure") (Hit :type "HitResult Structure (by ref)"))
  (bind _tempmesh (`self.TEMPmesh`))
  (if (!= HitComponent (`GameplayStatics.GetPlayerCharacter` 0))
    (`PrimitiveComponent.SetPhysicsLinearVelocity` _tempmesh (0.0 0.0 0.0) false "None")
    (`PrimitiveComponent.SetSimulatePhysics` _tempmesh false)))

(fn `UserConstructionScript`)