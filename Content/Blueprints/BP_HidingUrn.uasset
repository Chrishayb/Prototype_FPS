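; Interactable urn the player hides in for a limited time, which shatters when they leave.
; JumpIn hides the player, disables capsule collision and movement, teleports them above the urn, removes the outline, and starts a timer with a UMG countdown widget.
; Interacting again or timer expiry calls JumpOut, restoring the player, breaking the destructible mesh and ending interaction.
; Tick shows the interaction text while occupied and turns it toward the camera.
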(event `self.ReceiveBeginPlay`
  ;[1 1 1] BeginPlay
  (`SceneComponent.SetVisibility` (`self.InteractionText`) false false))

(event `self.ReciveInteractionStart`
  ;[1 1 1] Interacting
  (if (`self.isBeingUsed`)
    (`self.JumpOut`)
    (`self.EndInteraction`)
    (else
      (`self.JumpIn`)
      (`PlayerCharacter.SetInteractionTarget` (`self.PlayerReference`) self))))

(event `self.ReciveInteractionEnd`
  ;[1 1 1] End Interaction
  (`self.DisableInteractActor`))

(event `self.ReceiveTick`
  (params (DeltaSeconds :type "Float (single-precision)"))
  (bind _interactiontext (`self.InteractionText`))
  (if (`SceneComponent.IsVisible` _interactiontext)
    (`SceneComponent.K2_SetWorldRotation` (`self.InteractionText`) (`KismetMathLibrary.FindLookAtRotation` (`SceneComponent.K2_GetComponentLocation` _interactiontext) (`PlayerCameraManager.GetCameraLocation` (`PlayerController.PlayerCameraManager` (`GameplayStatics.GetPlayerController` 0)))) false false)
    (elif (`self.isBeingUsed`)
      (`SceneComponent.SetVisibility` (`self.InteractionText`) true false))))

(fn `JumpIn`
  (locals (NewLocalVar_0 :type "Vector Structure" :default (0.0 0.0 0.0)))
  (bind _returnvalue (`GameplayStatics.GetPlayerCharacter` 0))
  (bind _charactermovement (`Character.CharacterMovement` _returnvalue))
  (set `self.isBeingUsed` true)
  (set `self.WalkSpeed` (`CharacterMovementComponent.MaxWalkSpeed` _charactermovement))
  (set `CharacterMovementComponent.MaxWalkSpeed` 0.0 _charactermovement)
  (set `self.playerlocation` (`self.K2_GetActorLocation` _returnvalue))
  (`self.SetActorHiddenInGame` _returnvalue true)
  (`PrimitiveComponent.SetCollisionEnabled` (`Character.CapsuleComponent` _returnvalue) "NoCollision")
  (bind _output_get (set `self.NewVar_1` (`self.K2_GetActorLocation`)))
  (bind _output_get_2 (set `self.endlocation` (`KismetMathLibrary.MakeVector` (.x _output_get) (.y _output_get) (+ (.z _output_get) 200.0))))
  (`self.K2_SetActorLocation` _returnvalue _output_get_2 false true)
  (`ActorComponent.K2_DestroyComponent` (`self.Outline`))
  (`KismetSystemLibrary.K2_SetTimer` self "JumpOut" (`self.JumpOutTime`))
  (bind _returnvalue_2 (`|CreateWidget` "/Game/Blueprints/Widgets/WBP_UrnTimer.WBP_UrnTimer_C"))
  (`UserWidget.AddToViewport` _returnvalue_2 0)
  (set `self.TimerDestroy` _returnvalue_2))

(fn `JumpOut`
  (bind _returnvalue (`GameplayStatics.GetPlayerCharacter` 0))
  (bind _urndestructiblemesh (`self.UrnDestructibleMesh`))
  (bind _returnvalue_2 (`SceneComponent.K2_GetComponentLocation` _urndestructiblemesh))
  (set `self.isBeingUsed` false)
  (set `CharacterMovementComponent.MaxWalkSpeed` (`self.WalkSpeed`) (`Character.CharacterMovement` (`GameplayStatics.GetPlayerCharacter` 0)))
  (`self.K2_SetActorLocation` _returnvalue (`self.playerlocation`) false true)
  (`self.SetActorHiddenInGame` _returnvalue false)
  (`PrimitiveComponent.SetCollisionEnabled` (`Character.CapsuleComponent` _returnvalue) "QueryAndPhysics")
  (`SceneComponent.SetVisibility` (`self.InteractionText`) false false)
  (`self.EndInteraction`)
  (`Widget.RemoveFromParent` (`self.TimerDestroy`))
  (`KismetSystemLibrary.K2_ClearTimer` self "JumpOut")
  (`DestructibleComponent.ApplyDamage` _urndestructiblemesh 1.0 _returnvalue_2 _returnvalue_2 1.0)
  (`GameplayStatics.PlaySound2D` "/Game/Sound/GLASS_Fragment_03_mono_Cue.GLASS_Fragment_03_mono_Cue" 1.0 1.0 0.0 null null))

(fn `UserConstructionScript`)