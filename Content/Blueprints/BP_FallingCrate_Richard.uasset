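; Interactable falling crate that plays a fall animation and then becomes a physical blocker.
; The blocking collider starts disabled on BeginPlay; interaction start plays the animation, sets a timer that enables the collider shortly after, and ends the interaction.
; Interaction end disables further interaction with the actor.
; Overlap events and hint-text visibility and rotation logic are deprecated leftovers that do nothing.
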(event `self.ReceiveBeginPlay`
  ;[1 1 1] Disable the blocking collision
  (`PrimitiveComponent.SetCollisionEnabled` (`self.BlockedCollider`) "NoCollision"))

(event `self.ReciveInteractionStart`
  ;[1 1 1] On Interaction Start Event
  (`SkeletalMeshComponent.PlayAnimation` (`self.Mesh`) "/Game/Assets/FallingCrates/CrateFall_Anim.CrateFall_Anim" false)
  (`KismetSystemLibrary.K2_SetTimer` null "SpawnCollider" 0.8)
  (`self.EndInteraction`))

(event `self.ReciveInteractionEnd`
  ;[1 1 1] On Interaction End Event
  (`self.DisableInteractActor`))

(event `self.Box.OnComponentBeginOverlap`
  (params (OverlappedComponent :type "PrimitiveComponent Object Reference") (OtherActor :type "Actor Object Reference") (OtherComp :type "PrimitiveComponent Object Reference") (OtherBodyIndex :type Integer) (bFromSweep :type Boolean) (SweepResult :type "HitResult Structure (by ref)"))
  ;[1 1 1] Deprecated (Not in use) Setting visibility of the Interaction Hint Text
)

(event `self.Box.OnComponentEndOverlap`
  (params (OverlappedComponent :type "PrimitiveComponent Object Reference") (OtherActor :type "Actor Object Reference") (OtherComp :type "PrimitiveComponent Object Reference") (OtherBodyIndex :type Integer))
  ;[1 1 1] Deprecated (Not in use) Setting visibility of the Interaction Hint Text
)

(fn `SpawnCollider`
  (`PrimitiveComponent.SetCollisionEnabled` (`self.BlockedCollider`) "QueryAndPhysics"))

(fn `UserConstructionScript`)