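; BP_Tomato is a thrown tomato projectile that splats on whatever it hits.
; On BeginPlay it launches the FishKunai component with a physics impulse along the actor's forward vector, scaled by ProjectileSpeed.
; On hit it spawns a temporary splat decal oriented to the impact normal, plays a splat sound and destroys itself.
; A separate debug function logs the TriggerSphere location.
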(event `self.ReceiveBeginPlay`
  (`PrimitiveComponent.AddImpulse` (`self.FishKunai`) (* (`KismetMathLibrary.GetForwardVector` (`self.K2_GetActorRotation`)) (`self.ProjectileSpeed`)) "None" false))

(event `self.FishKunai.OnComponentHit`
  (params (HitComponent :type "PrimitiveComponent Object Reference") (OtherActor :type "Actor Object Reference") (OtherComp :type "PrimitiveComponent Object Reference") (NormalImpulse :type "Vector Structure") (Hit :type "HitResult Structure (by ref)"))
  (`GameplayStatics.SpawnDecalAtLocation` "/Game/Assets/Stall_Fruit/TomatoSplat_Mat.TomatoSplat_Mat" (50.0 50.0 50.0) (`SceneComponent.K2_GetComponentLocation` (`self.FishKunai`)) (`KismetMathLibrary.MakeRotationFromAxes` (`.ImpactNormal` (`GameplayStatics.BreakHitResult` Hit))) 5.0)
  (`GameplayStatics.PlaySoundAtLocation` "/Game/Sound/GORE_Splat_Hit_Bubbles_mono_Cue.GORE_Splat_Hit_Bubbles_mono_Cue" (`SceneComponent.K2_GetComponentLocation` (`self.FishKunai`)) (struct) 1.0 1.0 0.0 null null null)
  (`self.K2_DestroyActor`))

(fn `ShowTriggerDebugValue`
  (bind _triggersphere (`self.TriggerSphere`))
  (`VisualLoggerKismetLibrary.LogLocation` _triggersphere (`SceneComponent.K2_GetComponentLocation` _triggersphere) "" (struct :`B` 1.0 :`A` 1.0) 10.0 "VisLogBP" true))

(fn `UserConstructionScript`)