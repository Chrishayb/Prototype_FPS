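; BP_BirdViewCamera is an overhead camera actor that follows the player character along the world X axis.
; On BeginPlay it caches the player character and snaps to that X position, defaulting to zero when no player is found.
; Each Tick it refreshes the X from the player and moves itself there without sweep, keeping Y at zero and Z at the CameraHeight variable.
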(event `self.ReceiveBeginPlay`
  (bind _returnvalue (`GameplayStatics.GetPlayerCharacter` 0))
  ;[1 1 1] Find PLayer reference and set the location
  (`/Engine/EditorBlueprintResources/StandardMacros.IsValid` _returnvalue
    (:`Is Valid`
      (bind _output_get (set `self.PlayerRef` _returnvalue))
      (set `self.CameraLocationX` (.x (`self.K2_GetActorLocation` _output_get))))
    (:`Is Not Valid`
      (set `self.CameraLocationX` 0.0)))
  (`self.K2_SetActorLocation` (`KismetMathLibrary.MakeVector` (`self.CameraLocationX`) 0.0 (`self.CameraHeight`))))

(event `self.ReceiveTick`
  (params (DeltaSeconds :type "Float (single-precision)"))
  ;[1 1 1] Constantly move the camera to the player relavant location
  (if (`KismetSystemLibrary.IsValid` (`self.PlayerRef`))
    (`self.UpdatePlayerLocationX`))
  (`self.K2_SetActorLocation` (`KismetMathLibrary.MakeVector` (`self.CameraLocationX`) 0.0 (`self.CameraHeight`))))

(fn `UpdatePlayerLocationX`
  (set `self.CameraLocationX` (.x (`self.K2_GetActorLocation` (`self.PlayerRef`)))))

(fn `UserConstructionScript`)